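; Gun actor that snaps to the player's gun socket on Interact when it has no owner, and fires projectiles.
; FirePressed plays an ADS fire montage on the owner character, whose notify spawns BP_Projectile at the Muzzle socket.
; Projectile velocity points at the owner's look-at point, falling back to muzzle forward when absolute yaw delta reaches 90 degrees or more.
; The owner reference arrives separately through GetOwnerChar.
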(event Collision|EventActorBeginOverlap
  (params (OtherActor :type Actor%20Object%20Reference)))

(event EventTick
  (params (DeltaSeconds :type Float%20%28single-precision%29)))

(event EventInteract
  ;[1 1 1] Implement Interact Interface
  (Utilities|IsValid (Variables|Default|GetOwnerChar)
    (:Is%20Not%20Valid
      (Transformation|AttachComponentToComponent (Variables|/Script/Engine.Character|GetMesh (Game|GetPlayerCharacter 0)) "gun1Socket" "SnapToTarget" "SnapToTarget" "SnapToTarget" true))))

(event EventFirePressed
  ;[1 1 1] Fire
  (Animation|Montage|PlayMontage (Variables|/Script/Engine.Character|GetMesh (Variables|Default|GetOwnerChar)) "/Game/MyAssets/CharacterAnimation/A_2HW_ADS_Fire_Montage.A_2HW_ADS_Fire_Montage"
    (:OnNotifyBegin
      (bind _returnvalue (Game|SpawnActorfromClass "/Game/MyAssets/Blueprints/BP_Projectile.BP_Projectile_C" (Transformation|GetSocketTransform (Variables|Default|GetSkeletalMesh) "Muzzle" "RTS_World") "AlwaysSpawn" 0 0))
      (Variables|Default|SetProjectileRef _returnvalue)
      (bind _returnvalue_2 (Default|CalculateLookatPoint (Variables|Default|GetOwnerChar)))
      (Variables|Default|SetLookAtPoint _returnvalue_2)
      (Utilities|IsValid (Variables|Default|GetProjectileRef)
        (:Is%20Valid
          (Variables|/Script/Engine.MovementComponent|SetVelocity (Variables|/Game/MyAssets/Blueprints/BP_Projectile.BP_Projectile_C|GetProjectileMovement (Variables|Default|GetProjectileRef)) (* (select (>= (Math|Float|Absolute(Float) (Variables|/Game/MyAssets/Blueprints/BP_BaseChar.BP_BaseChar_C|GetDelta%20Value%20Z%20%28Yaw%29 (Variables|Default|GetOwnerChar))) 9e+01) (Math|Vector|GetForwardVector (Transformation|GetSocketRotation (Variables|Default|GetSkeletalMesh) "Muzzle")) (Math|Vector|Normalize (- (Variables|Default|GetLookAtPoint) (Transformation|GetSocketLocation (Variables|Default|GetSkeletalMesh) "Muzzle")))) (Variables|Default|GetProjectileVelocity))))))))

(event EventGetOwnerChar
  (params (OwnerChar :type BP%20Base%20Char%20Object%20Reference))
  ;[1 1 1] Fire
  (Variables|Default|SetOwnerChar OwnerChar))

(fn ConstructionScript)