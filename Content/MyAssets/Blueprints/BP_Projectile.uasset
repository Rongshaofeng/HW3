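; BP_Projectile is a projectile actor that damages what it hits and explodes.
; When SphereCollision hits, it applies point damage to the other actor, using its Damage value and the reversed velocity direction.
; If the hit component is valid, it adds a velocity-scaled impulse at the projectile's location, then spawns an explosion particle and destroys itself.
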(event OnComponentHit(SphereCollision)
  (params (HitComponent :type Primitive%20Component%20Object%20Reference) (OtherActor :type Actor%20Object%20Reference) (OtherComp :type Primitive%20Component%20Object%20Reference) (NormalImpulse :type Vector :default "0, 0, 0") (Hit :type Hit%20Result%20Structure%20%28by%20ref%29))
  (Game|Damage|ApplyPointDamage OtherActor (Variables|Default|GetDamage) (* (Math|Vector|Normalize (Transformation|GetVelocity)) -1.0) Hit)
  (Utilities|IsValid OtherComp
    (:Is%20Valid
      (Physics|AddImpulseatLocation OtherComp (* (Transformation|GetVelocity) 1e+01) (Transformation|GetActorLocation) "None")
      (Utilities|IsValid self
        (:Is%20Valid
          (Effects|SpawnEmitteratLocation "/Game/MobileStarterContent/Particles/P_Explosion.P_Explosion" (Transformation|GetActorLocation))
          (Actor|DestroyActor))))))

(fn ConstructionScript)