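; BP_EscapeEnemy is an enemy AI Blueprint in the EscapeAI folder, extending a parent class.
; On BeginPlay it runs the parent logic, hides PlayerUI and sets itself as OwnerActor on the AIHUD from its widget component.
; It then prints its HP as debug output.
; Tick is disabled and construction only calls the parent, so the file itself defines no escape behavior.
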(event EventBeginPlay
  (|CallParentFunction)
  (Widget|SetVisibility (Variables|Default|GetPlayerUI) "Hidden")
  (bind _asaihud (Utilities|Casting|CastToAIHUD (UserInterface|GetUserWidgetObject (Variables|Default|GetWidget))))
  (Variables|/Game/MyAssets/UMG/AIHUD.AIHUD_C|SetOwnerActor _asaihud self)
  (Development|PrintString (Utilities|String|ToString(Float) (Variables|Default|GetHP))))

(event Collision|EventActorBeginOverlap
  (params (OtherActor :type Actor%20Object%20Reference)))

(event EventTick
  (params (DeltaSeconds :type Float%20%28single-precision%29))
  (|CallParentFunction DeltaSeconds) ; This node is disabled and will not be called.\nDrag off pins to build functionality.
)

(fn ConstructionScript
  (|CallParentFunction))