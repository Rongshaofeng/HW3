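; AI enemy character that starts play armed with a gun and carries its own HUD widget.
; On BeginPlay it runs the parent logic, hides PlayerUI, then spawns a BP_WeaponGun with mesh collision disabled.
; It sets itself as the gun's owner, snaps it to gun1Socket on its mesh and calls EquipOrUnEquipWeapon.
; Finally, it registers itself as OwnerActor on the AIHUD in its widget component.
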(event EventBeginPlay
  (|CallParentFunction)
  (Widget|SetVisibility (Variables|Default|GetPlayerUI) "Hidden")
  (bind _returnvalue (Game|SpawnActorfromClass "/Game/MyAssets/Blueprints/BP_WeaponGun.BP_WeaponGun_C" (Transformation|GetActorTransform) "Undefined" 0 0))
  (bind _output_get (Variables|Default|SetWeaponGun1 _returnvalue))
  (Collision|SetCollisionEnabled (Variables|/Game/MyAssets/Blueprints/BP_WeaponGun.BP_WeaponGun_C|GetSkeletalMesh _output_get) "NoCollision")
  (Variables|/Game/MyAssets/Blueprints/BP_WeaponGun.BP_WeaponGun_C|SetOwnerChar _output_get self)
  (Transformation|AttachComponentToComponent _output_get (Variables|Character|GetMesh) "gun1Socket" "SnapToTarget" "SnapToTarget" "SnapToTarget" true)
  (CallFunction|EquiporUnEquipWeapon)
  (bind _asaihud (Utilities|Casting|CastToAIHUD (UserInterface|GetUserWidgetObject (Variables|Default|GetWidget))))
  (Variables|/Game/MyAssets/UMG/AIHUD.AIHUD_C|SetOwnerActor _asaihud self))

(event Collision|EventActorBeginOverlap
  (params (OtherActor :type Actor%20Object%20Reference)))

(event EventTick
  (params (DeltaSeconds :type Float%20%28single-precision%29))
  (|CallParentFunction DeltaSeconds) ; This node is disabled and will not be called.\nDrag off pins to build functionality.
)

(fn ConstructionScript
  (|CallParentFunction))